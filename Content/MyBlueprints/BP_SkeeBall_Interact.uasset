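; BP_SkeeBall_Interact is an interaction point that moves the player and their camera when E is pressed nearby, apparently for skee-ball.
; A sphere overlap with the third-person character shows the PressE prompt and opens a gate; leaving hides and closes it.
; While the gate is open, E calls MoveCamera on the player cached at BeginPlay and teleports them by a fixed world offset.
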(event `self.ReceiveBeginPlay`
  (bind _asbp_third_person_character (cast `/Game/ThirdPerson/Blueprints/BP_ThirdPersonCharacter` (`GameplayStatics.GetPlayerCharacter` 0)))
  (set `self.The Player` _asbp_third_person_character))

(event `E Pressed`
  (bind _the_player (`self.The Player`))
  (`/Engine/EditorBlueprintResources/StandardMacros.Gate` true :!label _label
    (:`Exit`
      (`/Game/ThirdPerson/Blueprints/BP_ThirdPersonCharacter.MoveCamera` _the_player)
      (`self.K2_AddActorWorldOffset` _the_player (0.0 -350.0 15.0) false true))))

(event `self.Sphere.OnComponentBeginOverlap`
  (params (OverlappedComponent :type "PrimitiveComponent Object Reference") (OtherActor :type "Actor Object Reference") (OtherComp :type "PrimitiveComponent Object Reference") (OtherBodyIndex :type Integer) (bFromSweep :type Boolean) (SweepResult :type "HitResult Structure (by ref)"))
  (cast `/Game/ThirdPerson/Blueprints/BP_ThirdPersonCharacter` OtherActor)
  (`SceneComponent.SetVisibility` (`self.PressE`) true false)
  (goto _label :!via `Open`))

(event `self.Sphere.OnComponentEndOverlap`
  (params (OverlappedComponent :type "PrimitiveComponent Object Reference") (OtherActor :type "Actor Object Reference") (OtherComp :type "PrimitiveComponent Object Reference") (OtherBodyIndex :type Integer))
  (cast `/Game/ThirdPerson/Blueprints/BP_ThirdPersonCharacter` OtherActor)
  (`SceneComponent.SetVisibility` (`self.PressE`) false false)
  (goto _label :!via `Close`))

(fn `UserConstructionScript`)