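; BP_Generator is an interactable generator that the player can use with a wrench to shut off electrified water.
; Entering its interaction volume shows a "Press E" prompt and opens a Gate that lets the E key through; leaving closes it.
; If the player has a wrench, pressing E breaks it and calls GeneratorOff on the BP_Electrified_Water actor found by class.
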(event `self.ReceiveBeginPlay`
  (bind _asbp_third_person_character (cast `/Game/ThirdPerson/Blueprints/BP_ThirdPersonCharacter` (`GameplayStatics.GetPlayerCharacter` 0)))
  (set `self.The Player` _asbp_third_person_character))

(event `Key|E`
  (params (Key :type "Key Structure"))
  (bind _the_player (`self.The Player`))
  (:`Pressed`
    (`/Engine/EditorBlueprintResources/StandardMacros.Gate` true :!label _label
      (:`Exit`
        (if (`/Game/ThirdPerson/Blueprints/BP_ThirdPersonCharacter.HasWrench` _the_player)
          (`/Game/ThirdPerson/Blueprints/BP_ThirdPersonCharacter.PlayMessage` _the_player "The Wrench Broke!" 2.0)
          (set `/Game/ThirdPerson/Blueprints/BP_ThirdPersonCharacter.HasWrench` false _the_player)
          (bind _returnvalue (`GameplayStatics.GetActorOfClass` "/Game/MyBlueprints/BP_Electrified_Water.BP_Electrified_Water_C"))
          (`/Game/MyBlueprints/BP_Electrified_Water.Generator_Off` _returnvalue))))))

(event `self.Generator_Interact_Space.OnComponentBeginOverlap`
  (params (OverlappedComponent :type "PrimitiveComponent Object Reference") (OtherActor :type "Actor Object Reference") (OtherComp :type "PrimitiveComponent Object Reference") (OtherBodyIndex :type Integer) (bFromSweep :type Boolean) (SweepResult :type "HitResult Structure (by ref)"))
  (cast `/Game/ThirdPerson/Blueprints/BP_ThirdPersonCharacter` OtherActor)
  (`/Game/ThirdPerson/Blueprints/BP_ThirdPersonCharacter.PlayMessage` (`self.The Player`) "Press E" 0.0)
  (goto _label :!via `Open`))

(event `self.Generator_Interact_Space.OnComponentEndOverlap`
  (params (OverlappedComponent :type "PrimitiveComponent Object Reference") (OtherActor :type "Actor Object Reference") (OtherComp :type "PrimitiveComponent Object Reference") (OtherBodyIndex :type Integer))
  (cast `/Game/ThirdPerson/Blueprints/BP_ThirdPersonCharacter` OtherActor)
  (goto _label :!via `Close`))

(fn `UserConstructionScript`)