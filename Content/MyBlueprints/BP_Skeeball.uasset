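; BP_Skeeball is a skeeball that is aimed in two timeline-driven stages and then launched with a physics impulse.
; SetAngle runs an angle timeline, and SetPower stops it and manually triggers its finish to start the power timeline.
; Both values are copied to the third-person player character, while power and angle form a Z-rotated vector.
; Fire enables gravity on the sphere and applies that vector as an impulse.
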(event `self.ReceiveTick`
  (params (DeltaSeconds :type "Float (single-precision)")))

(event `self.ReceiveBeginPlay`
  (bind _asbp_third_person_character (cast `/Game/ThirdPerson/Blueprints/BP_ThirdPersonCharacter` (`GameplayStatics.GetPlayerCharacter` 0)))
  (set `self.Player` _asbp_third_person_character))

(event `Set Angle`
  (bind _player (`self.Player`))
  (bind (_direction _angle) (`Timeline|Angle Timeline` :!via `PlayFromStart` :!label _label)
    (:`Update`
      (set `self.Timeline Stopped` false)
      (set `/Game/ThirdPerson/Blueprints/BP_ThirdPersonCharacter.Angle` _angle _player))
    (:`Finished`
      (if (`self.Timeline Stopped`)
        (bind (_direction_2 _power) (`Timeline|Power Timeline` :!via `PlayFromStart`)
          (:`Update`
            (set `/Game/ThirdPerson/Blueprints/BP_ThirdPersonCharacter.Power` _power _player)
            (set `self.rotatedVel` (`KismetMathLibrary.RotateAngleAxis` (`KismetMathLibrary.MakeVector` 0.0 _power) _angle (0.0 0.0 1.0)))))))))

(event `Set Power`
  (set `self.Timeline Stopped` true)
  (`self.Angle Timeline__FinishedFunc`)
  (goto _label :!via `Stop`))

(event `Fire`
  (bind _sphere (`self.Sphere`))
  (`PrimitiveComponent.SetEnableGravity` _sphere true)
  (`PrimitiveComponent.AddImpulse` _sphere (`self.rotatedVel`) "None" false))

(fn `UserConstructionScript`)