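; Elevator call button that the player presses with E to open the elevator doors.
; An overlap volume toggles a gate on the E input, and Tick shows a "Press E" prompt while the player is inside until the first press.
; A Timeline nudges the button mesh, then swaps the light ring and arrow decal material and opens the BP_Elevator_Doors found by class lookup.
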(event `self.ReceiveTick`
  (params (DeltaSeconds :type "Float (single-precision)"))
  (if (`self.In Bounds`)
    (if (not (`self.Button Pressed`))
      (`/Game/ThirdPerson/Blueprints/BP_ThirdPersonCharacter.PlayMessage` (`self.The Player`) "Press E" 1.0))))

(event `self.ReceiveBeginPlay`
  (bind _asbp_third_person_character (cast `/Game/ThirdPerson/Blueprints/BP_ThirdPersonCharacter` (`GameplayStatics.GetPlayerCharacter` 0)))
  (set `self.The Player` _asbp_third_person_character))

(event `E Pressed`
  (`/Engine/EditorBlueprintResources/StandardMacros.Gate` true :!label _label
    (:`Exit`
      (bind _returnvalue (`GameplayStatics.GetActorOfClass` "/Game/MyBlueprints/BP_Elevator_Doors.BP_Elevator_Doors_C"))
      (set `self.Button Pressed` true)
      (bind (_direction _newtrack_0) (`Timeline|Timeline`)
        (:`Update`
          (`SceneComponent.K2_AddRelativeLocation` (`self.Button`) (`KismetMathLibrary.MakeVector` 0.0 0.0 _newtrack_0) false false))
        (:`Finished`
          (`PrimitiveComponent.SetMaterial` (`self.Light Ring`) 0 "/Engine/VREditor/Teleport/TeleportDirectionMaterial.TeleportDirectionMaterial")
          (`PrimitiveComponent.SetMaterial` (`self.Arrow Decal`) 0 "/Engine/VREditor/Teleport/TeleportDirectionMaterial.TeleportDirectionMaterial")
          (`/Game/MyBlueprints/BP_Elevator_Doors.Open Door` _returnvalue))))))

(event `self.Button_Interact_Space.OnComponentBeginOverlap`
  (params (OverlappedComponent :type "PrimitiveComponent Object Reference") (OtherActor :type "Actor Object Reference") (OtherComp :type "PrimitiveComponent Object Reference") (OtherBodyIndex :type Integer) (bFromSweep :type Boolean) (SweepResult :type "HitResult Structure (by ref)"))
  (cast `/Game/ThirdPerson/Blueprints/BP_ThirdPersonCharacter` OtherActor)
  (set `self.In Bounds` true)
  (goto _label :!via `Open`))

(event `self.Button_Interact_Space.OnComponentEndOverlap`
  (params (OverlappedComponent :type "PrimitiveComponent Object Reference") (OtherActor :type "Actor Object Reference") (OtherComp :type "PrimitiveComponent Object Reference") (OtherBodyIndex :type Integer))
  (cast `/Game/ThirdPerson/Blueprints/BP_ThirdPersonCharacter` OtherActor)
  (set `self.In Bounds` false)
  (goto _label :!via `Close`))

(fn `UserConstructionScript`)