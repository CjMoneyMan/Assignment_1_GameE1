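; BP_Wrench is a wrench pickup that grants the player the item on overlap.
; It caches the third-person character at BeginPlay, and any collider overlap sets that character's HasWrench flag without checking the overlapping actor.
; The pickup then plays a sound at the player, spawns an attached fire emitter and destroys itself.
; A timeline meant to move and rotate the wrench meshes is present but never runs.
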(event `self.ReceiveBeginPlay`
  (bind _asbp_third_person_character (cast `/Game/ThirdPerson/Blueprints/BP_ThirdPersonCharacter` (`GameplayStatics.GetPlayerCharacter` 0)))
  (set `self.The Player` _asbp_third_person_character))

(event `self.Wrench_Collider.OnComponentBeginOverlap`
  (params (OverlappedComponent :type "PrimitiveComponent Object Reference") (OtherActor :type "Actor Object Reference") (OtherComp :type "PrimitiveComponent Object Reference") (OtherBodyIndex :type Integer) (bFromSweep :type Boolean) (SweepResult :type "HitResult Structure (by ref)"))
  (bind _the_player (`self.The Player`))
  (set `/Game/ThirdPerson/Blueprints/BP_ThirdPersonCharacter.HasWrench` true _the_player)
  (`GameplayStatics.PlaySoundAtLocation` "/Game/MySounds/Item_PickUp.Item_PickUp" (`self.K2_GetActorLocation` _the_player) (struct) 1.0 1.0 0.0 null null null null)
  (`GameplayStatics.SpawnEmitterAttached` "/Game/StarterContent/Particles/P_Fire.P_Fire")
  (`self.K2_DestroyActor`))

(fn `UserConstructionScript`)